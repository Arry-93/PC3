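; First-person player character that walks, looks around with clamped pitch, toggles a torch, and picks up and rotates interactable cubes.
; Grab line-traces from the camera for a BP_InteractableCube and disables its physics; releasing restores physics.
; While held, the cube is teleported to GrabPoint each Tick and rotated by secondary input axes.
; An earlier PhysicsHandle-based grab remains as disabled or unconnected nodes, and ObjectRoll is an empty stub.
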(event `InputAction|Grab`
  (params (Key :type "Key Structure"))
  (bind _camera (`self.Camera`))
  (bind _returnvalue (`SceneComponent.K2_GetComponentLocation` _camera))
  ;[1 1 1] Grab raycast and setting
  (:`Pressed`
    (if (not (`self.isGrabbing`))
      (bind (_outhit _returnvalue_2) (`KismetSystemLibrary.LineTraceSingle` :`Start` _returnvalue :`End` (+ _returnvalue (* (`SceneComponent.GetForwardVector` _camera) 300.0)) :`TraceChannel` "TraceTypeQuery2" :`DrawDebugType` "Persistent"))
      (if _returnvalue_2
        (bind (_bblockinghit _binitialoverlap _time _distance _location _impactpoint _normal _impactnormal _physmat _hitactor) (`GameplayStatics.BreakHitResult` _outhit))
        (bind _asbp_interactable_cube (cast `/Game/Blueprints/Interactable/BP_InteractableCube` _hitactor))
        (set `self.InspectedObj` _asbp_interactable_cube)
        (set `self.isGrabbing` true)
        (bind _cube (`/Game/Blueprints/Interactable/BP_InteractableCube.Cube` _asbp_interactable_cube))
        (`PrimitiveComponent.SetSimulatePhysics` _cube false))))
  (:`Released`
    (set `self.isGrabbing` false)
    (if (!= _hitactor null)
      (`PrimitiveComponent.SetSimulatePhysics` _cube true))))

(event `self.ReceiveTick`
  (params (DeltaSeconds :type "Float (single-precision)"))
  ;[1 1 1] Update grabbed object location
  (if (`self.isGrabbing`)
    (`self.K2_SetActorLocation` (`self.InspectedObj`) (`SceneComponent.K2_GetComponentLocation` (`self.GrabPoint`)) false false)))

(event `InputAxis|Horizontal2`
  (params (AxisValue :type "Float (single-precision)"))
  (bind _inspectedobj (`self.InspectedObj`))
  ;[1 1 1] Grabbed object rotation
  (if (`self.isGrabbing`)
    (if (!= _inspectedobj null)
      (`self.K2_AddActorLocalRotation` _inspectedobj (`KismetMathLibrary.MakeRotator` 0.0 0.0 AxisValue) false false))))

(event `InputAxis|MouseHorizontal`
  (params (AxisValue :type "Float (single-precision)"))
  ;[1 1 1] CameraMovement
  (`self.AddControllerYawInput` AxisValue))

(event `InputAxis|Vertical`
  (params (AxisValue :type "Float (single-precision)"))
  (bind (_returnvalue_roll _returnvalue_pitch _returnvalue_yaw) (`KismetMathLibrary.BreakRotator` (`self.GetControlRotation`)))
  ;[1 1 1] Movement
  (`self.AddMovementInput` (`KismetMathLibrary.GetForwardVector` (`KismetMathLibrary.MakeRotator` 0.0 0.0 _returnvalue_yaw)) AxisValue))

(event `InputAxis|MouseVertical`
  (params (AxisValue :type "Float (single-precision)"))
  ;[1 1 1] CameraMovement
  (`self.AddControllerPitchInput` AxisValue))

(event `InputAxis|Vertical2`
  (params (AxisValue :type "Float (single-precision)"))
  (bind _inspectedobj (`self.InspectedObj`))
  ;[1 1 1] Grabbed object rotation
  (if (`self.isGrabbing`)
    (if (!= _inspectedobj null)
      (`self.K2_AddActorLocalRotation` _inspectedobj (`KismetMathLibrary.MakeRotator` AxisValue) false false))))

(event `self.ReceiveBeginPlay`
  (bind _returnvalue (`GameplayStatics.GetPlayerCameraManager` 0))
  (bind _cameralimit (`self.CameraLimit`))
  ;[1 1 1] CameraMovement
  (set `PlayerCameraManager.ViewPitchMin` (- 0.0 _cameralimit) _returnvalue)
  (set `PlayerCameraManager.ViewPitchMax` _cameralimit _returnvalue))

(event `InputAxis|Horizontal`
  (params (AxisValue :type "Float (single-precision)"))
  (bind (_returnvalue_roll _returnvalue_pitch _returnvalue_yaw) (`KismetMathLibrary.BreakRotator` (`self.GetControlRotation`)))
  ;[1 1 1] Movement
  (`self.AddMovementInput` (`KismetMathLibrary.GetRightVector` (`KismetMathLibrary.MakeRotator` 0.0 0.0 _returnvalue_yaw)) AxisValue))

(event `InputAction|Torch`
  (params (Key :type "Key Structure"))
  (bind _torch (`self.Torch`))
  ;[1 1 1] Torch
  (:`Pressed`
    (`/Engine/EditorBlueprintResources/StandardMacros.FlipFlop`
      (:`A`
        (set `self._torch` true)
        (`SceneComponent.SetVisibility` _torch true false))
      (:`B`
        (set `self._torch` false)
        (`SceneComponent.SetVisibility` _torch false false)))))

(fn `Object roll`
  (params (NewParam :type Boolean)))

(fn `UserConstructionScript`)