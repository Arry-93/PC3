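; Placeholder door that the player removes by pressing the Action input while holding a key.
; A box trigger sets InsideTrigger on BP_Player when the player enters and clears it on exit.
; Tick reads that flag from the last cached player to enable or disable the door's input, and the Action press destroys the door if HasKey is true.
; Disabled and unconnected nodes from an earlier input setup remain in the graph.
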(event `self.ReceiveTick`
  (params (DeltaSeconds :type "Float (single-precision)"))
  (bind _returnvalue (`GameplayStatics.GetPlayerController` 0))
  (if (!= (stale `self.Box.OnComponentBeginOverlap` OtherActor) null)
    (if (`self.ActorHasTag` (stale `self.Box.OnComponentBeginOverlap` OtherActor) "Player")
      (if (`/Game/Blueprints/Characters/BP_Player.InsideTrigger` (stale `self.Box.OnComponentBeginOverlap` _asbp_player))
        (`self.EnableInput` _returnvalue)
        (else
          (`self.DisableInput` _returnvalue))))))

(event `self.Box.OnComponentBeginOverlap`
  (params (OverlappedComponent :type "PrimitiveComponent Object Reference") (OtherActor :type "Actor Object Reference") (OtherComp :type "PrimitiveComponent Object Reference") (OtherBodyIndex :type Integer) (bFromSweep :type Boolean) (SweepResult :type "HitResult Structure (by ref)"))
  (if (`self.ActorHasTag` OtherActor "Player")
    (bind _asbp_player (cast `/Game/Blueprints/Characters/BP_Player` OtherActor))
    (set `/Game/Blueprints/Characters/BP_Player.InsideTrigger` true _asbp_player)))

(event `InputAction|Action`
  (params (Key :type "Key Structure"))
  (:`Pressed`
    (if (`/Game/Blueprints/Characters/BP_Player.HasKey` (stale `self.Box.OnComponentBeginOverlap` _asbp_player))
      (`self.K2_DestroyActor`))))

(event `self.Box.OnComponentEndOverlap`
  (params (OverlappedComponent :type "PrimitiveComponent Object Reference") (OtherActor :type "Actor Object Reference") (OtherComp :type "PrimitiveComponent Object Reference") (OtherBodyIndex :type Integer))
  (bind _asbp_player (cast `/Game/Blueprints/Characters/BP_Player` OtherActor))
  (set `/Game/Blueprints/Characters/BP_Player.InsideTrigger` false _asbp_player))

(fn `UserConstructionScript`)